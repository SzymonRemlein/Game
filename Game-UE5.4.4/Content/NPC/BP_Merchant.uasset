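; BP_Merchant is a merchant NPC that sets its displayed name and starting money, then registers itself with AI_ControllerNeutral through a cast of its owner.
; While it sees the player, Tick feeds the NPC anim blueprint's LookAtPosition with a forward vector from interpolated NPC-to-player mesh rotations, not a world location.
; The Dialogue event hands off to DialogueSystem, while DialogueFirst and Calling are unused.
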(event `self.ReceiveTick`
  (params (DeltaSeconds :type "Float (single-precision)"))
  (if (`self.NPCseePlayer`)
    (bind _asbp_third_person_character (cast `/Game/ThirdPerson/Blueprints/BP_ThirdPersonCharacter` (`GameplayStatics.GetPlayerCharacter` 0)))
    (bind _asabp_npc_enemy (cast `/Game/NPC/Animation/ABP_NPC_ENEMY` (`SkeletalMeshComponent.GetAnimInstance` (`self.Mesh`))))
    (set `/Game/NPC/Animation/ABP_NPC_ENEMY.LookAtPosition` (`KismetMathLibrary.Conv_RotatorToVector` (`KismetMathLibrary.RInterpTo` (`SceneComponent.GetSocketRotation` (`self.Mesh`) "None") (`SceneComponent.GetSocketRotation` (`Character.Mesh` _asbp_third_person_character) "None") 100.0 100.0)) _asabp_npc_enemy)))

(event `self.beginPlayCon`
  (`/Game/HUD/WB_Inputs/WB_Name.setName` (`self.WB_Name`) "Merchant")
  (set `self.money` 1000)
  (bind _asai_controller_neutral (cast `/Game/NPC/AI/Neutrals/AI_ControllerNeutral` (`self.GetOwner`)))
  (set `/Game/NPC/AI/Neutrals/AI_ControllerNeutral.merchant` self _asai_controller_neutral))

(event `self.dialogue`
  ;[1 1 1] DIALOGUE
  (`self.dialogueSystem` _))

(fn `UserConstructionScript`)