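; Base NPC Blueprint with health, a name tag and an item inventory, with empty begin play, tick and dialogue hooks for child classes.
; Damage runs through the Statistic component, and defeat ragdolls the mesh and clears the enemy flag.
; Health and name widgets face the camera, while ChangeVisibility moves the player's click prompt over non-enemy or defeated NPCs.
; The construction script fills 30 item slots from data tables for the player's inventory panel.
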(event `self.ReceiveBeginPlay`
  (bind _statistic (`self.Statistic`))
  ;[1 1 1] BEGIN PLAY
  (bind _aswb_health (cast `/Game/HUD/WB_Player/WB_Health` (`WidgetComponent.GetWidget` (`self.HealthBar`))))
  (set `self.WB_Health` _aswb_health)
  (`/Game/ThirdPerson/Blueprints/Components/Statistic.set_Stats` _statistic (`self.stats`))
  (`/Game/ThirdPerson/Blueprints/Components/Statistic.healthBar` _statistic (`self.WB_Health`))
  (bind _aswb_name (cast `/Game/HUD/WB_Inputs/WB_Name` (`WidgetComponent.GetWidget` (`self.actorName`))))
  (set `self.WB_Name` _aswb_name)
  (bind _asbp_third_person_character (cast `/Game/ThirdPerson/Blueprints/BP_ThirdPersonCharacter` (`GameplayStatics.GetPlayerCharacter` 0)))
  (set `self.As BP Third Person Character` _asbp_third_person_character)
  (`self.beginPlayContinue`))

(event `beginPlayContinue`
  ;[1 1 1] BEGIN PLAY
  ;;[1 1 1] EMPTY FUNCTION TO OVERRIDE
)

(event `self.ReceiveTick`
  (params (DeltaSeconds :type "Float (single-precision)"))
  (bind _healthbar (`self.HealthBar`))
  (bind _actorname (`self.actorName`))
  ;[1 1 1] EVENT TICK AND EVENT  "TickContinue" FOR OTHER CLASS THAT INHERITED
  (`SceneComponent.K2_SetWorldRotation` _healthbar (`KismetMathLibrary.FindLookAtRotation` (`SceneComponent.K2_GetComponentLocation` _healthbar) (`SceneComponent.K2_GetComponentLocation` (`PlayerCameraManager.TransformComponent` (`GameplayStatics.GetPlayerCameraManager` 0)))) false false)
  (`SceneComponent.K2_SetWorldRotation` _actorname (`KismetMathLibrary.FindLookAtRotation` (`SceneComponent.K2_GetComponentLocation` _actorname) (`SceneComponent.K2_GetComponentLocation` (`PlayerCameraManager.TransformComponent` (`GameplayStatics.GetPlayerCameraManager` 0)))) false false)
  (`self.eventTickContinue`))

(event `eventTickContinue`
  ;[1 1 1] EVENT TICK AND EVENT  "TickContinue" FOR OTHER CLASS THAT INHERITED
)

(event `self.ReceiveAnyDamage`
  (params (Damage :type "Float (single-precision)") (DamageType :type "DamageType Object Reference") (InstigatedBy :type "Controller Object Reference") (DamageCauser :type "Actor Object Reference"))
  (bind _die (`/Game/ThirdPerson/Blueprints/Components/Statistic.DecreaseHealth` (`self.Statistic`) Damage))
  (bind _output_get (set `self.isBeat` _die))
  (if _output_get
    (`PrimitiveComponent.SetSimulatePhysics` (`self.Mesh`) true)
    (set `self.isEnemy` false)))

(event `/Game/ThirdPerson/Blueprints/I_dialogue.changeVisibility`
  (params (bool :type Boolean))
  (bind _returnvalue (`GameplayStatics.GetPlayerCharacter` 0))
  (bind (_returnvalue_x _returnvalue_y _returnvalue_z) (`KismetMathLibrary.BreakVector` (`SceneComponent.K2_GetComponentLocation` (`self.Mesh`))))
  (bind (_returnvalue_x_2 _returnvalue_y_2 _returnvalue_z_2) (`KismetMathLibrary.BreakVector` (`SceneComponent.K2_GetComponentLocation` (`self.CapsuleComponent`))))
  (bind _clickbutton (`/Game/ThirdPerson/Blueprints/BP_ThirdPersonCharacter.clickButton` (`self.As BP Third Person Character`)))
  (bind _clickbutton_2 (`/Game/ThirdPerson/Blueprints/BP_ThirdPersonCharacter.clickButton` (`self.As BP Third Person Character`)))
  (if (and bool (not (`self.isEnemy`)))
    (if (not (`self.isBeat`))
      (`SceneComponent.K2_SetWorldLocation` _clickbutton (`KismetMathLibrary.MakeVector` _returnvalue_x_2 _returnvalue_y_2 (+ _returnvalue_z_2 140.0)) false false)
      (`SceneComponent.SetVisibility` _clickbutton true false)
      (`SceneComponent.SetVisibility` (`self.actorName`) true false)
      (else
        (`SceneComponent.K2_SetWorldLocation` _clickbutton_2 (`KismetMathLibrary.MakeVector` _returnvalue_x _returnvalue_y (+ _returnvalue_z 140.0)) false false)
        (`SceneComponent.SetVisibility` _clickbutton_2 true false)
        (`SceneComponent.SetVisibility` (`self.actorName`) false false)
        (`SceneComponent.SetVisibility` (`self.HealthBar`) false false)))
    (else
      (bind _asbp_third_person_character (cast `/Game/ThirdPerson/Blueprints/BP_ThirdPersonCharacter` _returnvalue))
      (bind _clickbutton_3 (`/Game/ThirdPerson/Blueprints/BP_ThirdPersonCharacter.clickButton` _asbp_third_person_character))
      (`SceneComponent.K2_SetWorldLocation` _clickbutton_3 (`SceneComponent.K2_GetComponentLocation` (`Character.CapsuleComponent` _returnvalue)) false false)
      (`SceneComponent.SetVisibility` _clickbutton_3 false false)
      (`SceneComponent.SetVisibility` (`self.actorName`) false false))))

(event `OpenEQ`
  ;[1 1 1] INVENTROY
  (`/Game/HUD/WB_Inventory/WB_PlayerPanels.OtherEQ_panel` (`/Game/ThirdPerson/Blueprints/Components/Inventory.WB_Inventory` (`/Game/ThirdPerson/Blueprints/BP_ThirdPersonCharacter.Inventory` (`self.As BP Third Person Character`))) (`self.amountsItem`) (`self.itemTable`))
  (`SceneComponent.SetVisibility` (`/Game/ThirdPerson/Blueprints/BP_ThirdPersonCharacter.clickButton` (`self.As BP Third Person Character`)) false false))

(event `closeEQ`
  ;[1 1 1] INVENTROY
  (`/Game/ThirdPerson/Blueprints/Components/Inventory.Close Inventory` (`/Game/ThirdPerson/Blueprints/BP_ThirdPersonCharacter.Inventory` (`self.As BP Third Person Character`)))
  (`Widget.SetVisibility` (`/Game/HUD/WB_Inventory/WB_PlayerPanels.WB_InventoryPanel_Merchant` (`/Game/ThirdPerson/Blueprints/Components/Inventory.WB_Inventory` (`/Game/ThirdPerson/Blueprints/BP_ThirdPersonCharacter.Inventory` (`self.As BP Third Person Character`)))) "Hidden"))

(fn `dialogue`
  (return))

(fn `UserConstructionScript`
  (for _index (range 30)
    (bind _output (`|GetArrayItem` (`self.item_Informations`) _index))
    (bind _returnvalue (`|GetDataTableRow` (break `DataTableRowHandle` (break `/Game/Items/S_ItemD` _output)) (`.RowName` (break `DataTableRowHandle` (break `/Game/Items/S_ItemD` _output))))
      (:`then`
        (`KismetArrayLibrary.Array_Set` (`self.itemTable`) _index _returnvalue)))))