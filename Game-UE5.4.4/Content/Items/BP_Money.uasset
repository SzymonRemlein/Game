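; BP_Money is a money item that shows a value label in a widget component above its static mesh.
; BeginPlay writes its variable into the WB_Name widget and places the label using the mesh's bounds, while Tick rotates it toward the player camera.
; ChangeVisibility shows or hides the label along with the player character's ClickButton, moving that button above the mesh or back to the character.
; The Dialogue event is empty.
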(event `self.ReceiveBeginPlay`
  (bind _staticmesh (`self.StaticMesh`))
  (bind (_returnvalue_x _returnvalue_y) (`KismetMathLibrary.BreakVector` (`SceneComponent.K2_GetComponentLocation` _staticmesh)))
  (bind _aswb_name (cast `/Game/HUD/WB_Inputs/WB_Name` (`WidgetComponent.GetWidget` (`self.Value`))))
  (bind _output_get (set `self.WB_Name` _aswb_name))
  (`TextBlock.SetText` (`/Game/HUD/WB_Inputs/WB_Name.actorName` _output_get) (`KismetTextLibrary.Conv_StringToText` (`KismetStringLibrary.Conv_IntToString` (`self.variable`))))
  (`SceneComponent.K2_SetWorldLocation` (`self.Value`) (`KismetMathLibrary.MakeVector` _returnvalue_x _returnvalue_y (+ (.z (`.Max` (`StaticMeshComponent.GetLocalBounds` _staticmesh))) 75.0)) false false))

(event `self.ReceiveTick`
  (params (DeltaSeconds :type "Float (single-precision)"))
  (`SceneComponent.K2_SetWorldRotation` (`self.Value`) (`KismetMathLibrary.FindLookAtRotation` (`SceneComponent.K2_GetComponentLocation` (`self.Value`)) (`SceneComponent.K2_GetComponentLocation` (`PlayerCameraManager.TransformComponent` (`GameplayStatics.GetPlayerCameraManager` 0)))) false false))

(event `/Game/ThirdPerson/Blueprints/I_dialogue.dialogue`)

(event `/Game/ThirdPerson/Blueprints/I_dialogue.changeVisibility`
  (params (bool :type Boolean))
  (bind _returnvalue (`GameplayStatics.GetPlayerCharacter` 0))
  (bind _staticmesh (`self.StaticMesh`))
  (bind (_returnvalue_x _returnvalue_y) (`KismetMathLibrary.BreakVector` (`SceneComponent.K2_GetComponentLocation` _staticmesh)))
  (if bool
    (bind _asbp_third_person_character (cast `/Game/ThirdPerson/Blueprints/BP_ThirdPersonCharacter` (`GameplayStatics.GetPlayerCharacter` 0)))
    (bind _clickbutton (`/Game/ThirdPerson/Blueprints/BP_ThirdPersonCharacter.clickButton` _asbp_third_person_character))
    (`SceneComponent.K2_SetWorldLocation` _clickbutton (`KismetMathLibrary.MakeVector` _returnvalue_x _returnvalue_y (+ (.z (`.Max` (`StaticMeshComponent.GetLocalBounds` _staticmesh))) 125.0)) false false)
    (`SceneComponent.SetVisibility` _clickbutton true false)
    (`SceneComponent.SetVisibility` (`self.Value`) true false)
    (else
      (bind _asbp_third_person_character_2 (cast `/Game/ThirdPerson/Blueprints/BP_ThirdPersonCharacter` _returnvalue))
      (bind _clickbutton_2 (`/Game/ThirdPerson/Blueprints/BP_ThirdPersonCharacter.clickButton` _asbp_third_person_character_2))
      (`SceneComponent.K2_SetWorldLocation` _clickbutton_2 (`SceneComponent.K2_GetComponentLocation` (`Character.CapsuleComponent` _returnvalue)) false false)
      (`SceneComponent.SetVisibility` _clickbutton_2 false false)
      (`SceneComponent.SetVisibility` (`self.Value`) false false))))

(fn `UserConstructionScript`)