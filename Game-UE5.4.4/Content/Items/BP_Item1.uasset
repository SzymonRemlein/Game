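; BP_Item1 is an item actor that takes its name and mesh from an item struct, read from a data table row unless flagged as spawned.
; BeginPlay fills a name widget and positions it using the mesh's local bounds, and Tick turns it toward the camera.
; ChangeVisibility toggles that label and moves the player character's ClickButton over the item, or back to the player when hiding.
; The Dialogue function is empty.
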(event `self.ReceiveTick`
  (params (DeltaSeconds :type "Float (single-precision)"))
  (`SceneComponent.K2_SetWorldRotation` (`self.itemName`) (`KismetMathLibrary.FindLookAtRotation` (`SceneComponent.K2_GetComponentLocation` (`self.itemName`)) (`SceneComponent.K2_GetComponentLocation` (`PlayerCameraManager.TransformComponent` (`GameplayStatics.GetPlayerCameraManager` 0)))) false false))

(event `self.ReceiveBeginPlay`
  (bind _staticmesh (`self.StaticMesh`))
  (bind _item_s_name (break `/Game/Items/S_Item` (`self.item_s`)))
  (bind (_returnvalue_x _returnvalue_y) (`KismetMathLibrary.BreakVector` (`SceneComponent.K2_GetComponentLocation` _staticmesh)))
  (bind _aswb_name (cast `/Game/HUD/WB_Inputs/WB_Name` (`WidgetComponent.GetWidget` (`self.itemName`))))
  (bind _output_get (set `self.WB_Name` _aswb_name))
  (`TextBlock.SetText` (`/Game/HUD/WB_Inputs/WB_Name.actorName` _output_get) (`KismetTextLibrary.Conv_StringToText` _item_s_name))
  (`SceneComponent.K2_SetWorldLocation` (`self.itemName`) (`KismetMathLibrary.MakeVector` _returnvalue_x _returnvalue_y (+ (.z (`.Max` (`StaticMeshComponent.GetLocalBounds` _staticmesh))) 75.0)) false false))

(event `self.changeVisibility`
  (params (bool :type Boolean))
  (bind _returnvalue (`GameplayStatics.GetPlayerCharacter` 0))
  (bind _staticmesh (`self.StaticMesh`))
  (bind (_returnvalue_x _returnvalue_y) (`KismetMathLibrary.BreakVector` (`SceneComponent.K2_GetComponentLocation` _staticmesh)))
  (if bool
    (bind _asbp_third_person_character (cast `/Game/ThirdPerson/Blueprints/BP_ThirdPersonCharacter` (`GameplayStatics.GetPlayerCharacter` 0)))
    (bind _clickbutton (`/Game/ThirdPerson/Blueprints/BP_ThirdPersonCharacter.clickButton` _asbp_third_person_character))
    (`SceneComponent.K2_SetWorldLocation` _clickbutton (`KismetMathLibrary.MakeVector` _returnvalue_x _returnvalue_y (+ (.z (`.Max` (`StaticMeshComponent.GetLocalBounds` _staticmesh))) 125.0)) false false)
    (`SceneComponent.SetVisibility` _clickbutton true false)
    (`SceneComponent.SetVisibility` (`self.itemName`) true false)
    (else
      (bind _asbp_third_person_character_2 (cast `/Game/ThirdPerson/Blueprints/BP_ThirdPersonCharacter` _returnvalue))
      (bind _clickbutton_2 (`/Game/ThirdPerson/Blueprints/BP_ThirdPersonCharacter.clickButton` _asbp_third_person_character_2))
      (`SceneComponent.K2_SetWorldLocation` _clickbutton_2 (`SceneComponent.K2_GetComponentLocation` (`Character.CapsuleComponent` _returnvalue)) false false)
      (`SceneComponent.SetVisibility` _clickbutton_2 false false)
      (`SceneComponent.SetVisibility` (`self.itemName`) false false))))

(fn `dialogue`
  (return))

(fn `UserConstructionScript`
  (bind (_item_s_name _item_s_mesh) (break `/Game/Items/S_Item` (`self.item_s`)))
  (bind (_item_s_name_2 _item_s_mesh_2) (break `/Game/Items/S_Item` (`self.item_s`)))
  (bind _item_informations (`self.item_Informations`))
  (if (not (`self.isSpawned`))
    (bind _returnvalue (`|GetDataTableRow` (break `DataTableRowHandle` (break `/Game/Items/S_ItemD` _item_informations)) (`.RowName` (break `DataTableRowHandle` (break `/Game/Items/S_ItemD` _item_informations))))
      (:`then`
        (set `self.item_s` _returnvalue)
        (`StaticMeshComponent.SetStaticMesh` (`self.StaticMesh`) _item_s_mesh_2)))
    (else
      (`StaticMeshComponent.SetStaticMesh` (`self.StaticMesh`) _item_s_mesh))))