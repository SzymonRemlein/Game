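; BP_arrow is an arrow projectile that sticks into what it hits and damages BP_Template actors.
; On mesh overlap, it line-traces the hit component along the arrow's length to find the bone.
; It then stops physics and movement, snaps to that bone keeping world rotation, and on successful attach applies damage, with Head hits dealing less than others.
; Debug traces and prints remain active.
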(event `self.ReceiveBeginPlay`)

(event `self.ReceiveTick`
  (params (DeltaSeconds :type "Float (single-precision)")))

(event `self.StaticMesh.OnComponentBeginOverlap`
  (params (OverlappedComponent :type "PrimitiveComponent Object Reference") (OtherActor :type "Actor Object Reference") (OtherComp :type "PrimitiveComponent Object Reference") (OtherBodyIndex :type Integer) (bFromSweep :type Boolean) (SweepResult :type "HitResult Structure (by ref)"))
  (bind _staticmesh (`self.StaticMesh`))
  (bind _projectilemovement (`self.ProjectileMovement`))
  (bind _returnvalue (`SceneComponent.K2_GetComponentLocation` _staticmesh))
  (bind _returnvalue_2 (`SceneComponent.GetForwardVector` _staticmesh))
  (bind (_min _max) (`StaticMeshComponent.GetLocalBounds` _staticmesh))
  (if (!= OtherComp self)
    (bind (_hitlocation _hitnormal _bonename _outhit _returnvalue_3) (`PrimitiveComponent.K2_LineTraceComponent` SweepResult_HitComponent (+ _returnvalue (* _returnvalue_2 (.x _min))) (+ _returnvalue (* _returnvalue_2 (.x _max))) true true true))
    (if _returnvalue_3
      (`KismetSystemLibrary.PrintString` "GOWNA")
      (bind (_bblockinghit _binitialoverlap _time _distance _location _impactpoint _normal _impactnormal _physmat _hitactor _hitcomponent _hitbonename) (`GameplayStatics.BreakHitResult` _outhit))
      (`KismetSystemLibrary.PrintString` (`KismetStringLibrary.Concat_StrStr` (`KismetSystemLibrary.GetDisplayName` _hitactor) ": " (`KismetStringLibrary.Conv_NameToString` _hitbonename)))
      (`PrimitiveComponent.SetSimulatePhysics` (`self.StaticMesh`) false)
      (`MovementComponent.StopMovementImmediately` _projectilemovement)
      (set `ProjectileMovementComponent.ProjectileGravityScale` 0.0 _projectilemovement)
      (bind _returnvalue_4 (`SceneComponent.K2_AttachToComponent` (`self.StaticMesh`) _hitcomponent _hitbonename "SnapToTarget" "KeepWorld" "KeepWorld" true))
      (if _returnvalue_4
        (switch `name` _hitbonename
          (:`Default`
            (bind _asbp_template (cast `/Game/NPC/BP_Template` _hitactor))
            (`GameplayStatics.ApplyDamage` _asbp_template 100.0))
          (:`head`
            (bind _asbp_template_2 (cast `/Game/NPC/BP_Template` _hitactor))
            (`GameplayStatics.ApplyDamage` _asbp_template_2 10.0)))))))

(fn `UserConstructionScript`)