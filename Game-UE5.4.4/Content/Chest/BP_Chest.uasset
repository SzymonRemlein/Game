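; BP_Chest is an interactable loot chest that shows its contents in the player's inventory UI.
; A Box hit sets Front, which gates ChangeVisibility placing the player's click prompt above the chest and showing a camera-facing "Chest" label.
; The construction script fills ItemTable from data table rows.
; openChest and closeChest toggle the animation blueprint's open flag, prompt visibility and the inventory panels, passing items and amounts on opening.
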(event `self.ReceiveBeginPlay`
  (bind _aswb_name (cast `/Game/HUD/WB_Inputs/WB_Name` (`WidgetComponent.GetWidget` (`self.itemName`))))
  (bind _output_get (set `self.As WB Name` _aswb_name))
  (`/Game/HUD/WB_Inputs/WB_Name.setName` _output_get "Chest")
  (bind _asbp_third_person_character (cast `/Game/ThirdPerson/Blueprints/BP_ThirdPersonCharacter` (`GameplayStatics.GetPlayerCharacter` 0)))
  (set `self.As BP Third Person Character` _asbp_third_person_character))

(event `self.ReceiveTick`
  (params (DeltaSeconds :type "Float (single-precision)"))
  (`SceneComponent.K2_SetWorldRotation` (`self.itemName`) (`KismetMathLibrary.FindLookAtRotation` (`SceneComponent.K2_GetComponentLocation` (`self.itemName`)) (`SceneComponent.K2_GetComponentLocation` (`PlayerCameraManager.TransformComponent` (`GameplayStatics.GetPlayerCameraManager` 0)))) false false))

(event `/Game/ThirdPerson/Blueprints/I_dialogue.changeVisibility`
  (params (bool :type Boolean))
  (bind _returnvalue (`GameplayStatics.GetPlayerCharacter` 0))
  (bind (_returnvalue_x _returnvalue_y _returnvalue_z) (`KismetMathLibrary.BreakVector` (`SceneComponent.K2_GetComponentLocation` (`self.Chest`))))
  (if (and bool (`self.front`))
    (bind _asbp_third_person_character (cast `/Game/ThirdPerson/Blueprints/BP_ThirdPersonCharacter` (`GameplayStatics.GetPlayerCharacter` 0)))
    (bind _clickbutton (`/Game/ThirdPerson/Blueprints/BP_ThirdPersonCharacter.clickButton` _asbp_third_person_character))
    (`SceneComponent.K2_SetWorldLocation` _clickbutton (`KismetMathLibrary.MakeVector` _returnvalue_x _returnvalue_y (+ _returnvalue_z 220.0)) false false)
    (`SceneComponent.SetVisibility` _clickbutton true false)
    (`SceneComponent.SetVisibility` (`self.itemName`) true false)
    (else
      (bind _asbp_third_person_character_2 (cast `/Game/ThirdPerson/Blueprints/BP_ThirdPersonCharacter` _returnvalue))
      (bind _clickbutton_2 (`/Game/ThirdPerson/Blueprints/BP_ThirdPersonCharacter.clickButton` _asbp_third_person_character_2))
      (`SceneComponent.K2_SetWorldLocation` _clickbutton_2 (`SceneComponent.K2_GetComponentLocation` (`Character.CapsuleComponent` _returnvalue)) false false)
      (`SceneComponent.SetVisibility` _clickbutton_2 false false)
      (`SceneComponent.SetVisibility` (`self.itemName`) false false)
      (set `self.front` false))))

(event `self.Box.OnComponentHit`
  (params (HitComponent :type "PrimitiveComponent Object Reference") (OtherActor :type "Actor Object Reference") (OtherComp :type "PrimitiveComponent Object Reference") (NormalImpulse :type "Vector Structure") (Hit :type "HitResult Structure (by ref)"))
  (set `self.front` true))

(event `openChest`
  ;[1 1 1] OPEN AND CLOSE CHEST
  (bind _asabp_chest (cast `/Game/Chest/source/ABP_Chest` (`SkeletalMeshComponent.GetAnimInstance` (`self.Chest`))))
  (set `/Game/Chest/source/ABP_Chest.chestIsOpen?` true _asabp_chest)
  (`/Game/HUD/WB_Inventory/WB_PlayerPanels.OtherEQ_panel` (`/Game/ThirdPerson/Blueprints/Components/Inventory.WB_Inventory` (`/Game/ThirdPerson/Blueprints/BP_ThirdPersonCharacter.Inventory` (`self.As BP Third Person Character`))) (`self.amountsItem`) (`self.itemTable`))
  (`SceneComponent.SetVisibility` (`/Game/ThirdPerson/Blueprints/BP_ThirdPersonCharacter.clickButton` (`self.As BP Third Person Character`)) false false)
  (`SceneComponent.SetVisibility` (`self.itemName`) false false)
  (set `self.front` false))

(event `closeChest`
  ;[1 1 1] OPEN AND CLOSE CHEST
  (bind _asabp_chest (cast `/Game/Chest/source/ABP_Chest` (`SkeletalMeshComponent.GetAnimInstance` (`self.Chest`))))
  (set `/Game/Chest/source/ABP_Chest.chestIsOpen?` false _asabp_chest)
  (`SceneComponent.SetVisibility` (`/Game/ThirdPerson/Blueprints/BP_ThirdPersonCharacter.clickButton` (`self.As BP Third Person Character`)) true false)
  (`SceneComponent.SetVisibility` (`self.itemName`) true false)
  (`/Game/ThirdPerson/Blueprints/Components/Inventory.Close Inventory` (`/Game/ThirdPerson/Blueprints/BP_ThirdPersonCharacter.Inventory` (`self.As BP Third Person Character`)))
  (`Widget.SetVisibility` (`/Game/HUD/WB_Inventory/WB_PlayerPanels.WB_InventoryPanel_Merchant` (`/Game/ThirdPerson/Blueprints/Components/Inventory.WB_Inventory` (`/Game/ThirdPerson/Blueprints/BP_ThirdPersonCharacter.Inventory` (`self.As BP Third Person Character`)))) "Hidden")
  (set `self.front` true))

(fn `UserConstructionScript`
  (for _index (range 30)
    (bind _output (`|GetArrayItem` (`self.item_Informations`) _index))
    (bind _returnvalue (`|GetDataTableRow` (break `DataTableRowHandle` (break `/Game/Items/S_ItemD` _output)) (`.RowName` (break `DataTableRowHandle` (break `/Game/Items/S_ItemD` _output))))
      (:`then`
        (`KismetArrayLibrary.Array_Set` (`self.itemTable`) _index _returnvalue)))))